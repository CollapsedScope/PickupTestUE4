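; BP_ThrownItem is a projectile actor for a thrown pickup item that turns into a pickup when it comes to rest.
; When the ProjectileMovement stops, it spawns a BP_PickupWidget at its transform, sets ItemToAdd to its PickupClass and destroys itself.
; SetMeshFromPickup looks unfinished: it spawns an owned PickupClass actor if the class is valid, but never sets a mesh.
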(event `self.ProjectileMovement.OnProjectileStop`
  (params (ImpactResult :type "HitResult Structure (by ref)"))
  (bind _returnvalue (`|SpawnActorFromClass` "/Game/PickupTest/Blurprints/BP_PickupWidget.BP_PickupWidget_C" (`self.GetTransform`) "Undefined" "OverrideRootScale" null null))
  (set `/Game/PickupTest/Blurprints/BP_PickupWidget.ItemToAdd` (`self.PickupClass`) _returnvalue)
  (`self.K2_DestroyActor`))

(fn `SetMeshFromPickup`
  (if (`KismetSystemLibrary.IsValidClass` (`self.PickupClass`))
    (bind _returnvalue (`|SpawnActorFromClass` (`self.PickupClass`) (`self.GetTransform`) "Undefined" "OverrideRootScale" self null))))

(fn `UserConstructionScript`)