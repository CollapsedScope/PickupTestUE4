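; BP_PickupWidget is a pickup actor that displays an item and offers it to a nearby player character.
; On BeginPlay it spawns ItemToAdd at its own transform, doubled in scale and yawed 90 degrees.
; Collider overlaps by any actor toggle the PickupWidget prompt.
; For BP_PickupCharacterMaster they also set or clear the attached item and name, assign this actor as CurrentReferredWidget either way, and print the name.
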(event `self.ReceiveBeginPlay`
  (bind _itemtoadd (`self.ItemToAdd`))
  (if (`KismetSystemLibrary.IsValidClass` _itemtoadd)
    (bind _returnvalue (`|SpawnActorFromClass` _itemtoadd (`self.GetTransform`) "Undefined" "OverrideRootScale" null null))
    (`self.SetActorScale3D` _returnvalue (2.0 2.0 2.0))
    (`self.K2_SetActorRotation` _returnvalue (struct :`Pitch` 90.0) false)))

(event `self.Collider.OnComponentBeginOverlap`
  (params (OverlappedComponent :type "PrimitiveComponent Object Reference") (OtherActor :type "Actor Object Reference") (OtherComp :type "PrimitiveComponent Object Reference") (OtherBodyIndex :type Integer) (bFromSweep :type Boolean) (SweepResult :type "HitResult Structure (by ref)"))
  (`SceneComponent.SetVisibility` (`self.PickupWidget`) true false)
  (bind _asbp_pickup_character_master (cast `/Game/PickupTest/Blurprints/BP_PickupCharacterMaster` OtherActor))
  (set `/Game/PickupTest/Blurprints/BP_PickupCharacterMaster.AttachedItem` (`self.ItemToAdd`) _asbp_pickup_character_master)
  (bind _output_get (set `/Game/PickupTest/Blurprints/BP_PickupCharacterMaster.EquippedItemName` (`KismetSystemLibrary.GetObjectName` self) _asbp_pickup_character_master))
  (set `/Game/PickupTest/Blurprints/BP_PickupCharacterMaster.CurrentReferredWidget` self _asbp_pickup_character_master)
  (`KismetSystemLibrary.PrintString` _output_get))

(event `self.Collider.OnComponentEndOverlap`
  (params (OverlappedComponent :type "PrimitiveComponent Object Reference") (OtherActor :type "Actor Object Reference") (OtherComp :type "PrimitiveComponent Object Reference") (OtherBodyIndex :type Integer))
  (`SceneComponent.SetVisibility` (`self.PickupWidget`) false false)
  (bind _asbp_pickup_character_master (cast `/Game/PickupTest/Blurprints/BP_PickupCharacterMaster` OtherActor))
  (set `/Game/PickupTest/Blurprints/BP_PickupCharacterMaster.AttachedItem` null _asbp_pickup_character_master)
  (bind _output_get (set `/Game/PickupTest/Blurprints/BP_PickupCharacterMaster.EquippedItemName` "" _asbp_pickup_character_master))
  (set `/Game/PickupTest/Blurprints/BP_PickupCharacterMaster.CurrentReferredWidget` self _asbp_pickup_character_master)
  (`KismetSystemLibrary.PrintString` _output_get))

(fn `UserConstructionScript`)